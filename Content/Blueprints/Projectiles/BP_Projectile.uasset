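; Projectile Blueprint that damages whatever it hits and removes itself after a limited lifetime.
; Tick accumulates elapsed time in LifeTime and destroys the actor once it exceeds LifeExpectancy.
; The Hit event passes the other actor to DamagingPlayer, which applies DamageAmount and destroys the projectile, with no check that the target is a player.
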(event `self.ReceiveTick`
  (params (DeltaSeconds :type "Float (single-precision)"))
  (bind _output_get (set `self.LifeTime` (+ DeltaSeconds (`self.LifeTime`))))
  (if (> _output_get (`self.LifeExpectancy`))
    (`self.K2_DestroyActor`)))

(event `self.ReceiveHit`
  (params (MyComp :type "PrimitiveComponent Object Reference") (Other :type "Actor Object Reference") (OtherComp :type "PrimitiveComponent Object Reference") (bSelfMoved :type Boolean) (HitLocation :type "Vector Structure") (HitNormal :type "Vector Structure") (NormalImpulse :type "Vector Structure") (Hit :type "HitResult Structure (by ref)"))
  (`self.DamagingPlayer` Other))

(fn `DamagingPlayer`
  (params (DamagedActor :type "Actor Object Reference"))
  (`GameplayStatics.ApplyDamage` DamagedActor (`self.DamageAmount`))
  (`self.K2_DestroyActor`))

(fn `UserConstructionScript`)