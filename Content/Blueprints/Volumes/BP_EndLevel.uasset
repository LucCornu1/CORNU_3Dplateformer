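; BP_EndLevel is a level-exit volume that advances the game when the player overlaps it and no BP_Key actors remain in the level.
; It copies the player's score and health into BP_BaseGameInstance, then waits briefly before completing the level.
; Completion finds the current level in the LevelNames array and opens the next entry, or quits the game on the last.
; Despite its name, KeyRemaining returns true when no keys are left.
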(event `self.ReceiveActorBeginOverlap`
  (params (OtherActor :type "Actor Object Reference"))
  (`/Game/Libraries/BP_ActorMacroLibrary.IsPlayer` OtherActor
    (:`IsPlayer`
      (if (`self.KeyRemaining`)
        (`self.StorePlayerScore`)
        (`self.StorePlayerHealth`)
        (`KismetSystemLibrary.Delay` 2.0)
        (`self.CompleteLevel`)))))

(fn `CompleteLevel`
  (if (`self.IsFinalLevel`)
    (`KismetSystemLibrary.QuitGame` null "Quit")
    (else
      (`self.LoadNextLevel`))))

(fn `GetCurrentLevelIndex`
  (returns (ReturnValue :type Integer))
  (bind _returnvalue (`GameplayStatics.GetCurrentLevelName` true))
  (return (`KismetArrayLibrary.Array_Find` (`self.LevelNames`) (`KismetStringLibrary.Conv_StringToName` _returnvalue))))

(fn `GetLevelName`
  (returns (ReturnValue :type Name))
  (return (`|GetArrayItem` (`self.LevelNames`) (+ (`self.GetCurrentLevelIndex`) 1))))

(fn `IsFinalLevel`
  (returns (ReturnValue :type Boolean))
  (return (== (`KismetArrayLibrary.Array_LastIndex` (`self.LevelNames`)) (`self.GetCurrentLevelIndex`))))

(fn `KeyRemaining`
  (returns (ReturnBoolean :type Boolean))
  (bind _outactors (`GameplayStatics.GetAllActorsOfClass` "/Game/Blueprints/Collectables/BP_Key.BP_Key_C"))
  (return (<= (`KismetArrayLibrary.Array_Length` _outactors) 0)))

(fn `LoadNextLevel`
  (`GameplayStatics.OpenLevel` (`self.GetLevelName`)))

(fn `StorePlayerHealth`
  (bind _asbp_player_character (cast `/Game/Blueprints/Characters/BP_PlayerCharacter` (`GameplayStatics.GetPlayerCharacter` 0)))
  (bind _asbp_base_game_instance (cast `/Game/Blueprints/GameInstances/BP_BaseGameInstance` (`GameplayStatics.GetGameInstance`)))
  (set `/Game/Blueprints/GameInstances/BP_BaseGameInstance.PlayerHealth_GI` (`/Game/Blueprints/Characters/BP_PlayerCharacter.GetPlayerHealth` _asbp_player_character) _asbp_base_game_instance))

(fn `StorePlayerScore`
  (bind _asbp_player_character (cast `/Game/Blueprints/Characters/BP_PlayerCharacter` (`GameplayStatics.GetPlayerCharacter` 0)))
  (bind _asbp_base_game_instance (cast `/Game/Blueprints/GameInstances/BP_BaseGameInstance` (`GameplayStatics.GetGameInstance`)))
  (set `/Game/Blueprints/GameInstances/BP_BaseGameInstance.PlayerScore_GI` (`/Game/Blueprints/Characters/BP_PlayerCharacter.GetPlayerScore` _asbp_player_character) _asbp_base_game_instance))

(fn `UserConstructionScript`)