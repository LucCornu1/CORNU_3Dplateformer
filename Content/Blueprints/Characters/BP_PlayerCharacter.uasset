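; Player character Blueprint that manages the HUD, pause menu toggle, camera fades and level restart.
; BeginPlay builds the HUD and fades in; OnHitBP refreshes the life bar, and CameraFadeBP fades out once, then reloads the level.
; Tick applies damage below a Z border.
; Movement, look, jump and death logic is left disconnected, with input axis and AnyDamage events empty, alongside largely unused helper functions.
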(event `self.CameraFade_BP`
  (`/Engine/EditorBlueprintResources/StandardMacros.DoOnce` false
    (:`Completed`
      (bind _returnvalue (`self.StartCameraFadeOut`))
      (`KismetSystemLibrary.Delay` _returnvalue)
      (`self.RestartCurrentLevel`))))

(event `self.ReceiveTick`
  (params (DeltaSeconds :type "Float (single-precision)"))
  ;[0 0 0] CheckPlayerLocation
  (`self.CheckPositionZ`))

(event `self.OnHit_BP`
  (`/Game/UI/W_PlayerHud.Change Life Bar` (`self.PlayerHUD`) (`self.GetCurrentHealth`)))

(event `self.ReceiveAnyDamage`
  (params (Damage :type "Float (single-precision)") (DamageType :type "DamageType Object Reference") (InstigatedBy :type "Controller Object Reference") (DamageCauser :type "Actor Object Reference"))
  ;[1 0 0.02745] AnyDamageEvent
)

(event `InputAxis|Turn` :overrideparent false
  (params (AxisValue :type "Float (single-precision)"))
  ;[1 0 0.02745] Camera_MouseControl
)

(event `self.ReceiveBeginPlay`
  ;[0.7763 0.2317 1] AddingHUD
  (`self.CreateWidgetHUD`)
  ;[0.3065 0.3381 1] Camera Fade on BeginPlay method
  (`self.StartCameraFadeIn`)
  (`WidgetBlueprintLibrary.SetInputMode_GameOnly` (`GameplayStatics.GetPlayerController` 0))
  (bind _asbp_base_game_instance (cast `/Game/Blueprints/GameInstances/BP_BaseGameInstance` (`GameplayStatics.GetGameInstance`))))

(event `InputAxis|LookUp` :overrideparent false
  (params (AxisValue :type "Float (single-precision)"))
  ;[1 0 0.02745] Camera_MouseControl
)

(event `InputAction|Pause` :paused true
  (params (Key :type "Key Structure"))
  (:`Pressed`
    (`/Engine/EditorBlueprintResources/StandardMacros.FlipFlop`
      (:`A`
        (`WidgetLayoutLibrary.RemoveAllWidgets`)
        (`self.CreatePauseHUD`))
      (:`B`
        (`WidgetLayoutLibrary.RemoveAllWidgets`)
        (`self.CreateWidgetHUD`)
        (`GameplayStatics.SetGamePaused` false)
        (set `PlayerController.bShowMouseCursor` false (`GameplayStatics.GetPlayerController` 0))
        (`/Game/UI/W_PlayerHud.Change Life Bar` (`self.PlayerHUD`) (`self.GetCurrentHealth`))))))

(event `InputAxis|MoveForward` :consume false :overrideparent false
  (params (AxisValue :type "Float (single-precision)"))
  ;[1 0 0.02745] MovementInput_Handler
)

(event `InputAxis|MoveRight` :consume false :overrideparent false
  (params (AxisValue :type "Float (single-precision)"))
  ;[1 0 0.02745] MovementInput_Handler
)

(event `InputAction|Walk` :overrideparent false
  (params (Key :type "Key Structure"))
  ;[1 0 0.02745] MovementWalk
)

(event `InputAction|Jump`
  (params (Key :type "Key Structure"))
  ;[1 0 0.02745] MovementJump
)

(fn `AddMovementForward`
  (params (ScaleValue :type "Float (double-precision)"))
  (bind (_returnvalue_x _returnvalue_y) (`KismetMathLibrary.BreakVector` (`self.GetActorForwardVector`)))
  (`self.AddMovementInput` (`KismetMathLibrary.MakeVector` _returnvalue_x _returnvalue_y) ScaleValue))

(fn `AddMovementRight`
  (params (ScaleValue :type "Float (double-precision)"))
  (bind (_returnvalue_x _returnvalue_y) (`KismetMathLibrary.BreakVector` (`self.GetActorRightVector`)))
  (`self.AddMovementInput` (`KismetMathLibrary.MakeVector` _returnvalue_x _returnvalue_y) ScaleValue))

(fn `CheckPositionZ`
  (bind (_returnvalue_x _returnvalue_y _returnvalue_z) (`KismetMathLibrary.BreakVector` (`SceneComponent.K2_GetComponentLocation` (`self.CapsuleComponent`))))
  (if (<= _returnvalue_z (`self.WorldZBorder`))
    (`GameplayStatics.ApplyDamage` self 10.0)))

(fn `CreatePauseHUD`
  (returns (ReturnValue :type "/Game/UI/W_PauseHud Object Reference"))
  (bind _returnvalue (`|CreateWidget` "/Game/UI/W_PauseHud.W_PauseHud_C"))
  (`UserWidget.AddToViewport` _returnvalue 0)
  (return _returnvalue))

(fn `CreateWidgetHUD`
  (bind _returnvalue (`|CreateWidget` "/Game/UI/W_PlayerHud.W_PlayerHud_C" null self))
  (bind _output_get (set `self.PlayerHUD` _returnvalue))
  (`UserWidget.AddToViewport` _output_get 0))

(fn `GetPlayerHealth`
  (returns (PlayerHealth :type "Float (double-precision)"))
  (return 0.0))

(fn `GetPlayerScore`
  (returns (PlayerScore :type Integer))
  (return (`self.PlayerScore`)))

(fn `IncreasePlayerScore`
  (`/Engine/EditorBlueprintResources/StandardMacros.IncrementInt` (`self.PlayerScore`)))

(fn `IsAlive`
  (returns (ReturnValue :type Boolean))
  (return (not (`self.IsDead`))))

(fn `MouseX_Control`
  (params (Value :type "Float (double-precision)"))
  (`self.AddControllerYawInput` (`KismetMathLibrary.FClamp` Value -2.0 2.0)))

(fn `MouseY_Control`
  (params (Value :type "Float (double-precision)"))
  (`self.AddControllerPitchInput` (* (`KismetMathLibrary.FClamp` Value -0.4 0.4) -1.0)))

(fn `MovementForward`
  (if (`self.IsWalking`)
    (bind _output_get (set `self.AxisX` (`KismetMathLibrary.FClamp` (`self.AxisX`) -0.5 0.5)))
    (`self.AddMovementForward` _output_get)
    (else
      (`self.AddMovementForward` (`self.AxisX`)))))

(fn `MovementRight`
  (if (`self.IsWalking`)
    (bind _output_get (set `self.AxisY` (`KismetMathLibrary.FClamp` (`self.AxisY`) -0.5 0.5)))
    (`self.AddMovementRight` _output_get)
    (else
      (`self.AddMovementRight` (`self.AxisY`)))))

(fn `RestartCurrentLevel`
  (bind _returnvalue (`GameplayStatics.GetCurrentLevelName` true))
  (`GameplayStatics.OpenLevel` (`KismetStringLibrary.Conv_StringToName` _returnvalue)))

(fn `StartCameraFadeIn`
  (returns (ReturnValue :type "Float (double-precision)"))
  (`PlayerCameraManager.StartCameraFade` :`self` (`GameplayStatics.GetPlayerCameraManager` 0) :`FromAlpha` 1.0 :`Duration` 2.0 :`bHoldWhenFinished` true)
  (return 2.0))

(fn `StartCameraFadeOut`
  (returns (ReturnValue :type "Float (double-precision)"))
  (`PlayerCameraManager.StartCameraFade` :`self` (`GameplayStatics.GetPlayerCameraManager` 0) :`ToAlpha` 1.0 :`Duration` 2.0 :`bHoldWhenFinished` true)
  (return 2.0))

(fn `UserConstructionScript`)