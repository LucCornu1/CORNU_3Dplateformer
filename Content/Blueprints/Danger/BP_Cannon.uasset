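; BP_Cannon is a hazard actor that automatically fires projectiles on a repeating cycle from BeginPlay.
; After a fire-rate delay, it spawns a scaled BP_Projectile at the ProjectileSpawnPoint's world location and rotation.
; The CannonFire timeline then animates recoil by driving the Cannon component's relative Y location.
; The timeline's Cannon Fired event track loops execution back to the delay for the next shot.
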(event `self.ReceiveBeginPlay`
  (`KismetSystemLibrary.Delay` (`self.CannonFireRate`) :!label _label)
  (`self.SpawnProjectile`)
  (bind (_direction _cannon_recoil) (`Timeline|CannonFire` :!via `PlayFromStart`)
    (:`Update`
      (`self.CannonRecoil` _cannon_recoil))
    (:`Cannon Fired`
      (goto _label))))

(fn `CannonRecoil`
  (params (CannonYLocation :type "Float (double-precision)"))
  (`SceneComponent.K2_SetRelativeLocation` (`self.Cannon`) (`KismetMathLibrary.MakeVector` 0.0 CannonYLocation) false false))

(fn `SpawnProjectile`
  (bind _projectilespawnpoint (`self.ProjectileSpawnPoint`))
  (`|SpawnActorFromClass` "/Game/Blueprints/Projectiles/BP_Projectile.BP_Projectile_C" (`KismetMathLibrary.MakeTransform` (`SceneComponent.K2_GetComponentLocation` _projectilespawnpoint) (`SceneComponent.K2_GetComponentRotation` _projectilespawnpoint) (`KismetMathLibrary.Conv_DoubleToVector` (`self.ProjectileScale`))) "Undefined" "OverrideRootScale" null null))

(fn `UserConstructionScript`)